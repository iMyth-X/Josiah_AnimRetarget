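; Josiah Carter character actor, puppeteered by an interactor through tracked body data and input-driven facial states.
; Each Tick copies hip offsets and yaw to JosiahCarter_AnimBP and moves hand and foot target components to stored world transforms.
; BeginPlay enables player 0 input, which sets talking and held emotion flags (happy, angry, sad, shocked).
; The construction script attaches FeetCollider to the skeletal mesh's hips socket.
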(event EventBeginPlay
  ;[1 1 1] Wrangle Keyboard control from the game to this character
  (Input|EnableInput (Game|GetPlayerController 0)))

(event EventTick
  (params (DeltaSeconds :type Float%20%28single-precision%29))
  ;[1 1 1] Interactor gets position and orientation from puck and send it to the AnimBP
  (Utilities|FlowControl|Sequence
    (:then_0
      (bind _asjosiah_carter_anim_bp (Utilities|Casting|CastToJosiahCarter_AnimBP (Components|SkeletalMesh|GetAnimInstance (Variables|Default|GetSkeletalMesh))))
      (Utilities|IsValid _asjosiah_carter_anim_bp
        (:Is%20Valid
          (Variables|/Game/Characters/JosiahCarter/BluePrints/JosiahCarter_AnimBP.JosiahCarter_AnimBP_C|SetHipsY _asjosiah_carter_anim_bp (Variables|Default|GetHipsYVal))
          (Variables|/Game/Characters/JosiahCarter/BluePrints/JosiahCarter_AnimBP.JosiahCarter_AnimBP_C|SetHipsX _asjosiah_carter_anim_bp (Variables|Default|GetHipsXVal))
          (Variables|/Game/Characters/JosiahCarter/BluePrints/JosiahCarter_AnimBP.JosiahCarter_AnimBP_C|SetHipsYaw _asjosiah_carter_anim_bp (Variables|Default|GetHipsYaw)))
        (:Is%20Not%20Valid
          (Development|PrintString "Interactor Not Cast Correctly"))))
    (:then_1
      ;[1 1 1] Set the Position & Orientation of the Targets
      ;;[1 0.02 0.02] Left Hand
      (Transformation|SetWorldLocationAndRotation (Variables|Default|GetLHandScene) (Variables|Default|GetlHandPosition) (Variables|Default|GetLHandOrientation) false false)
      ;;[0.04035 1 0.03873] Right Hand
      (Transformation|SetWorldLocationAndRotation (Variables|Default|GetRHandScene) (Variables|Default|GetRHandPosition) (Variables|Default|GetRHandOrientation) false false)
      ;;[0 0 0] Left Foot
      (Transformation|SetWorldLocationAndRotation (Variables|Default|GetLFootScene) (Variables|Default|GetLFootPosition) (Variables|Default|GetLFootOrientation) false false)
      ;;[1 1 1] Right Foot
      (Transformation|SetWorldLocationAndRotation (Variables|Default|GetRFoot) (Variables|Default|GetRFootPosition) (Variables|Default|GetRFootOrientation) false false))))

(event Input|ActionEvents|InputActionInteractor_Happy
  (params (Key :type Key%20Structure :default "AnyKey"))
  ;[1 1 1] Face ANimation/States
  (:Pressed
    (Variables|Default|SetIsHappyBP true))
  (:Released
    (Variables|Default|SetIsHappyBP false)))

(event Input|ActionEvents|InputActionInteractor_Mad
  (params (Key :type Key%20Structure :default "AnyKey"))
  ;[1 1 1] Face ANimation/States
  (:Pressed
    (Variables|Default|SetIsAngryBP true))
  (:Released
    (Variables|Default|SetIsAngryBP false)))

(event Input|ActionEvents|InputActionInteractor_Sad
  (params (Key :type Key%20Structure :default "AnyKey"))
  ;[1 1 1] Face ANimation/States
  (:Pressed
    (Variables|Default|SetIsSadBP true))
  (:Released
    (Variables|Default|SetIsSadBP false)))

(event Input|ActionEvents|InputActionInteractor_Shock
  (params (Key :type Key%20Structure :default "AnyKey"))
  ;[1 1 1] Face ANimation/States
  (:Pressed
    (Variables|Default|SetIsShockedBP true))
  (:Released
    (Variables|Default|SetIsShockedBP false)))

(event Input|AxisEvents|InputAxisInteractorTalking
  (params (AxisValue :type Float%20%28single-precision%29))
  ;[1 1 1] Face ANimation/States
  (Variables|Default|SetIsTalkBP (Math|Conversions|ToBoolean(Integer) (Math|Float|Ceil AxisValue))))

(fn ConstructionScript
  ;[1 1 1] Remove the feet collider and attach to hips
  (Transformation|AttachComponentToComponent (Variables|Default|GetFeetCollider) (Variables|Default|GetSkeletalMesh) "HipsSocket" "KeepRelative" "KeepRelative" "KeepRelative" false))