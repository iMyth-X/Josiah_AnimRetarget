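; JosiahCarter character Blueprint that mirrors the pose of a MyExoRed mesh through tracker proxy components, apparently for full-body IK.
; Each tick it passes hip, shoulder, hand and foot positions to its Anim Blueprint, then moves the proxies to MyExoRed's sockets with swapped axes and offsets.
; Tracked-device reads, the limb target math and the shoulder effector update are present but unconnected.
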(event EventBeginPlay
  ;[1 1 1] Key Binding for Testing
  (Input|EnableInput (Game|GetPlayerController 0)))

(event EventTick
  (params (DeltaSeconds :type Float%20%28single-precision%29))
  ;[1 1 1] Sequence from Event Tick - Likley a temp measure
  (Utilities|FlowControl|Sequence
    (:then_0
      ;[1 1 1] Send positions to anim BP
      (bind _asjosiah_carter_lighthouse_anim (Utilities|Casting|CastToJosiahCarter_lighthouseAnim (Components|SkeletalMesh|GetAnimInstance (Variables|Default|GetSkeletalMesh))))
      (bind _selfout (|SetHips _asjosiah_carter_lighthouse_anim)
        (:execOut
          (bind _selfout_2 (|SetShoulders _selfout)
            (:execOut
              (bind _selfout_3 (|SetLeftArm _selfout_2)
                (:execOut
                  (bind _selfout_4 (|SetLeftLeg _selfout_3)
                    (:execOut
                      (bind _selfout_5 (|SetRightArm _selfout_4)
                        (:execOut
                          (|SetRightLeg _selfout_5))))))))))))
    (:then_1
      (|CollapseGraph_0))))

(fn ConstructionScript)